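; BP_Cylinder is an actor whose Pin component rises or sinks vertically according to how far the player pawn is from it.
; Every tick it normalizes that distance against MaxDistance, samples CurveAsset with it and raises the result to the Influence exponent.
; The shaped value is remapped to a clamped relative Z offset centered on zero, so the curve and exponent define the falloff.
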(event EventBeginPlay)

(event EventTick
  (params (DeltaSeconds :type Float%20%28single-precision%29))
  (Transformation|SetRelativeLocation (Variables|Default|GetPin) (Math|Vector|MakeVector 0.0 0.0 (Math|Float|MapRangeClamped (Math|Float|Power (Math|Curves|GetFloatValue (Variables|Default|GetCurveAsset) (Math|Float|MapRangeClamped (Math|Vector|VectorLength (- (Transformation|GetActorLocation (Game|Player|GetPlayerPawn 0)) (Transformation|GetActorLocation))) 0.0 (Variables|Default|GetMaxDistance) 0.0 1.0)) (Variables|Default|GetInfluence)) 0.0 1.0 -2.4e+02 2.4e+02)) false false))

(fn ConstructionScript)